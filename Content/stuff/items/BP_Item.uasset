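; BP_Item is a pickup actor that places an item object into the player's inventory on contact.
; On BeginPlay, it fills an unset ItemObject from GetDefaultItemObject, which is an empty stub here.
; When a BP_ThirdPersonCharacter overlaps its capsule, it passes ItemObject to that character's inventory component through TryAddItem.
; The actor destroys itself only if the add succeeds.
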(event OnComponentBeginOverlap(Capsule)
  (params (OverlappedComponent :type Primitive%20Component%20Object%20Reference) (OtherActor :type Actor%20Object%20Reference) (OtherComp :type Primitive%20Component%20Object%20Reference) (OtherBodyIndex :type Integer) (bFromSweep :type Boolean) (SweepResult :type Hit%20Result%20Structure%20%28by%20ref%29))
  (bind _asbp_third_person_character (Utilities|Casting|CastToBP_ThirdPersonCharacter OtherActor))
  (bind _added_ (Default|TryAddItem (Variables|/Game/ThirdPerson/Blueprints/BP_ThirdPersonCharacter.BP_ThirdPersonCharacter_C|Getinvcomp _asbp_third_person_character) (Variables|Default|GetItemObject)))
  (if _added_
    (Actor|DestroyActor)))

(event EventBeginPlay
  (Variables|Default|GetItemObject
    (:then)
    (:else
      (bind _itemobject (CallFunction|GetDefaultItemObject))
      (Variables|Default|SetItemObject _itemobject))))

(fn ConstructionScript)

(fn GetDefaultItemObject
  (return 0))