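; BP_ItemObject represents an item with grid-style dimensions, an icon, an item class and a rotation state.
; Rotate toggles the Rotated flag, which IsRotated reports.
; When rotated, GetDimentions returns the X and Y dimensions swapped and GetIcon returns the separate IconRotated asset instead of Icon.
; GetItemClass exposes the stored class regardless of rotation.
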(fn GetDimentions
  (bind _dimentions (Variables|Default|GetDimentions))
  (if (Variables|Default|GetRotated?)
    (return (Utilities|Struct|MakeIntPoint (.y _dimentions) (.x _dimentions)))
    (else
      (return (Variables|Default|GetDimentions)))))

(fn GetIcon
  (return (select (Variables|Default|GetRotated?) (Variables|Default|GetIconRotated) (Variables|Default|GetIcon))))

(fn GetItemClass
  (return (Variables|Default|GetItemClass)))

(fn Rotate
  (Variables|Default|SetRotated? (not (Variables|Default|GetRotated?))))

(fn IsRotated
  (return (Variables|Default|GetRotated?)))